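; Player controller for the sniper game that sets up UI, input mode and camera based on the current level.
; On the main menu level it shows the menu with cursor and UI-only input.
; Elsewhere it uses game-only input, adds a third-person reticle, and spawns a BP_PlayerCamera attached to the character as follow target and view target.
; A WinScreen event shows the win widget and restores cursor and UI input.
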(event Custom|WinScreen
  (bind _self self)
  ;[0.15 0.15 0.15 0.5] Win Screen
  (bind _returnvalue (UserInterface|CreateWidget "/Game/SS_SNIPERGAME/SS_BLUEPRINTS/SS_WIDGETS/WBP_WinScreen.WBP_WinScreen_C"))
  (UserInterface|Viewport|AddtoViewport _returnvalue 0)
  (Input|SetInputModeUIOnly _self _returnvalue "DoNotLock" false)
  (Variables|Default|SetbShowMouseCursor _self true))

(event EventBeginPlay
  (bind _returnvalue (Game|GetPlayerCharacter 0))
  (bind _self self)
  (bind _returnvalue_2 (Game|GetCurrentLevelName true))
  (if (Utilities|Enum|Equal(Enum) _returnvalue_2 "LVL_MAINMENU")
    ;[0.15 0.15 0.15 0.5] Create Main Menu
    (bind _returnvalue_3 (UserInterface|CreateWidget "/Game/SS_SNIPERGAME/SS_BLUEPRINTS/SS_WIDGETS/WBP_MainMenu.WBP_MainMenu_C" _self))
    (UserInterface|Viewport|AddtoViewport _returnvalue_3 0)
    (Input|SetInputModeUIOnly _self _returnvalue_3 "DoNotLock" false)
    (Variables|Default|SetbShowMouseCursor self true)
    (else
      ;[0.15 0.15 0.15 0.5] Remove Mouse Cursor
      (Variables|Default|SetbShowMouseCursor false)
      (Input|SetInputModeGameOnly self false)
      ;[0.15 0.15 0.15 0.5] Create 3rd Person Reticle
      (bind _returnvalue_4 (UserInterface|CreateWidget "/Game/SS_SNIPERGAME/SS_BLUEPRINTS/SS_WIDGETS/WBP_3RDPERSON_Reticle.WBP_3RDPERSON_Reticle_C"))
      (bind _output_get (Variables|Default|SetReticleWidget _returnvalue_4))
      (UserInterface|Viewport|AddtoViewport _output_get 0)
      ;[0.15 0.15 0.15 0.5] Camera Follows Character
      (bind _returnvalue_5 (Game|SpawnActorfromClass "/Game/SS_SNIPERGAME/SS_BLUEPRINTS/BP_PlayerCamera.BP_PlayerCamera_C" (Math|Conversions|ToTransform(Vector) (+ (Transformation|GetActorLocation _returnvalue) (* (Transformation|GetActorForwardVector _returnvalue) -4e+02))) "Undefined" "MultiplyWithRoot" 0 0))
      (Transformation|AttachActorToActor _returnvalue_5 _returnvalue "None" "SnapToTarget" "KeepWorld" "KeepWorld" false)
      (bind _output_get_2 (Variables|Default|SetPlayerCamera _returnvalue_5))
      (Variables|/Game/SS_SNIPERGAME/SS_BLUEPRINTS/BP_PlayerCamera.BP_PlayerCamera_C|SetFollowTarget _output_get_2 _returnvalue)
      (Game|Player|SetViewTargetwithBlend _output_get_2 0.0 "VTBlend_Linear" 0.0 false))))

(event EventTick
  (params (DeltaSeconds :type Float%20%28single-precision%29)))

(fn ConstructionScript)
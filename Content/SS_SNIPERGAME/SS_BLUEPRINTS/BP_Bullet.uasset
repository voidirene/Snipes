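; BP_Bullet is the sniper game's projectile, built from a collision Sphere and a ProjectileMovement component.
; On BeginPlay the sphere ignores its owner while moving.
; On hit, it stops and deactivates its movement, then destroys the other actor if it is a BP_Enemy.
; Hitting a BP_BOSS shows the win screen through BP_PlayerController before destroying the boss.
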(event OnComponentHit(Sphere)
  (params (HitComponent :type Primitive%20Component%20Object%20Reference) (OtherActor :type Actor%20Object%20Reference) (OtherComp :type Primitive%20Component%20Object%20Reference) (NormalImpulse :type Vector :default "0, 0, 0") (Hit :type Hit%20Result%20Structure%20%28by%20ref%29))
  (bind _projectilemovement (Variables|Default|GetProjectileMovement))
  (Utilities|FlowControl|Sequence
    (:then_0
      ;[0.15 0.15 0.15 0.5] Bullet Stops on hit
      (Development|PrintString "HIT")
      (Components|Movement|StopMovementImmediately _projectilemovement)
      (Components|Activation|Deactivate _projectilemovement))
    (:then_1
      (bind _asbp_enemy (Utilities|Casting|CastToBP_Enemy OtherActor))
      (Actor|DestroyActor _asbp_enemy))
    (:then_2
      (bind _asbp_boss (Utilities|Casting|CastToBP_BOSS OtherActor))
      (bind _asbp_player_controller (Utilities|Casting|CastToBP_PlayerController (Game|GetPlayerController 0)))
      (Default|WinScreen _asbp_player_controller)
      (Actor|DestroyActor _asbp_boss))))

(event EventBeginPlay
  (Collision|IgnoreActorwhenMoving (Variables|Default|GetSphere) (Components|GetOwner) true))

(event Collision|EventActorBeginOverlap
  (params (OtherActor :type Actor%20Object%20Reference)))

(event EventTick
  (params (DeltaSeconds :type Float%20%28single-precision%29)))

(fn ConstructionScript)
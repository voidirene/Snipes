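; BP_PlayerCamera is the sniper game's player camera actor, rotating each tick to match the follow target's control rotation.
; It switches between third-person and aim-down-sights cameras by activating one and deactivating the other.
; A timeline fades a dynamic invert post-process material on both cameras, and disabling the effect zeroes its weight.
; Camera travel detaches the actor, lerps it to a target location, then fires a finished dispatcher.
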(event Custom|Enter%20ADS
  ;[0.15 0.15 0.15 0.5] Swapping Camera Views
  (Components|Activation|Deactivate (Variables|Default|Get3rd_Person))
  (Components|Activation|Activate (Variables|Default|GetADS_Camera) false))

(event Custom|Exit%20ADS
  ;[0.15 0.15 0.15 0.5] Swapping Camera Views
  (Components|Activation|Deactivate (Variables|Default|GetADS_Camera))
  (Components|Activation|Activate (Variables|Default|Get3rd_Person) false))

(event Custom|Camera_Travel
  (params (TargetLocation :type Vector) (TravelDuration :type Float%20%28double-precision%29))
  ;[0.15 0.15 0.15 0.5] CAM TRAVEL EVENT
  (Transformation|DetachFromActor "KeepWorld" "KeepWorld" "KeepWorld")
  (Variables|Default|SetCameraStartLocation (Transformation|GetActorLocation))
  (Variables|Default|SetCameraTargetLocation TargetLocation)
  (bind _travelalpha (Timeline|TL_CameraTravel PlayFromStart)
    (:Update
      (Transformation|SetActorLocation (Math|Vector|Lerp(Vector) (Variables|Default|GetCameraStartLocation) (Variables|Default|GetCameraTargetLocation) _travelalpha) false false))
    (:Finished
      (Default|CallOnCameraTravelFinished))))

(event Custom|SetInvertEffect
  (params (Enabled :type Boolean))
  (bind _slowmaterial (Variables|Default|GetSlowMaterial))
  (if Enabled
    (CallFunction|StartInvertEffect)
    (else
      (Utilities|FlowControl|Sequence
        (:then_0
          (bind _invertalpha (Timeline|TL_InvertEffect Stop)
            (:Update
              (Rendering|Material|SetScalarParameterValue _slowmaterial "ABC" _invertalpha :!class /Script/Engine.MaterialInstanceDynamic)
              (Rendering|AddorUpdateBlendable (Variables|Default|Get3rd_Person) _slowmaterial _invertalpha :!class /Script/Engine.CameraComponent)
              (Rendering|AddorUpdateBlendable (Variables|Default|GetADS_Camera) (Variables|Default|GetSlowMaterial) _invertalpha :!class /Script/Engine.CameraComponent))))
        (:then_1
          (Rendering|AddorUpdateBlendable (Variables|Default|Get3rd_Person) (Variables|Default|GetSlowMaterial) 0.0 :!class /Script/Engine.CameraComponent)
          (Rendering|AddorUpdateBlendable (Variables|Default|GetADS_Camera) (Variables|Default|GetSlowMaterial) 0.0 :!class /Script/Engine.CameraComponent))))))

(event Custom|StartInvertEffect
  (bind _slowmaterial (Variables|Default|GetSlowMaterial))
  (bind _invertalpha (Timeline|TL_InvertEffect PlayFromStart)
    (:Update
      (Rendering|Material|SetScalarParameterValue _slowmaterial "ABC" _invertalpha :!class /Script/Engine.MaterialInstanceDynamic)
      (Rendering|AddorUpdateBlendable (Variables|Default|Get3rd_Person) _slowmaterial _invertalpha :!class /Script/Engine.CameraComponent)
      (Rendering|AddorUpdateBlendable (Variables|Default|GetADS_Camera) (Variables|Default|GetSlowMaterial) _invertalpha :!class /Script/Engine.CameraComponent))))

(event EventBeginPlay
  (bind _returnvalue (Rendering|Material|CreateDynamicMaterialInstance "/Game/SS_SNIPERGAME/SS_MATERIALS/TEST_PP_INVERTED.TEST_PP_INVERTED" "None" "None" :!class /Script/Engine.KismetMaterialLibrary))
  (bind _output_get (Variables|Default|SetSlowMaterial _returnvalue))
  (Rendering|AddorUpdateBlendable (Variables|Default|Get3rd_Person) _output_get 0.0 :!class /Script/Engine.CameraComponent)
  (Rendering|AddorUpdateBlendable (Variables|Default|GetADS_Camera) (Variables|Default|GetSlowMaterial) 0.0 :!class /Script/Engine.CameraComponent))

(event Collision|EventActorBeginOverlap
  (params (OtherActor :type Actor%20Object%20Reference)))

(event EventTick
  (params (DeltaSeconds :type Float%20%28single-precision%29))
  ;[0.15 0.15 0.15 0.5] Follows Player
  (Transformation|SetActorRotation (Pawn|GetControlRotation (Pawn|GetController (Variables|Default|GetFollowTarget)) :!class /Script/Engine.Controller)))

(fn ConstructionScript)
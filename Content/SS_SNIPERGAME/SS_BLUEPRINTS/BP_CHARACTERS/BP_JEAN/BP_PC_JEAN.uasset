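; Player character Jean for a sniper game, with movement, aim-down-sights, held slow motion, a timeline-lerped dash and teleport to the fired bullet.
; On BeginPlay it spawns the equipped weapon with a scope and attaches it to a mesh socket.
; Firing traces from the PlayerController's camera to aim a BP_Bullet spawned at ProjectileSpawn, with debug drawing.
; Only one bullet stays active: refiring replaces it, and teleporting moves Jean there and destroys it.
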(event EventBeginPlay
  (bind _returnvalue (Actor|GetActorOfClass "/Script/Engine.HUD"))
  (Variables|Default|SetHUD _returnvalue)
  (CallFunction|PlayerDefaults))

(event Input|ActionEvents|InputActionSHOOT
  (params (Key :type Key%20Structure))
  (bind _activebullet (Variables|Default|GetActiveBullet))
  ;[0.15 0.15 0.15 0.5] ACTIONS
  (:Pressed
    (Utilities|IsValid _activebullet
      (:Is%20Valid
        (Actor|DestroyActor _activebullet)
        (CallFunction|FIREBullet))
      (:Is%20Not%20Valid
        (CallFunction|FIREBullet)))))

(event Input|ActionEvents|InputActionTELEPORT
  (params (Key :type Key%20Structure))
  (bind _activebullet (Variables|Default|GetActiveBullet))
  ;[0.15 0.15 0.15 0.5] ACTIONS
  (:Pressed
    (Utilities|IsValid _activebullet
      (:Is%20Valid
        (Transformation|SetActorLocation (Transformation|GetActorLocation _activebullet) false true)
        (Actor|DestroyActor _activebullet)))))

(event Input|ActionEvents|InputActionSLOW
  (params (Key :type Key%20Structure))
  ;[0.15 0.15 0.15 0.5] ACTIONS
  (:Pressed
    (Utilities|Time|SetGlobalTimeDilation 0.2))
  (:Released
    (Utilities|Time|SetGlobalTimeDilation 1.0)))

(event Input|ActionEvents|InputActionDASH
  (params (Key :type Key%20Structure))
  ;[0.15 0.15 0.15 0.5] ACTIONS
  (:Pressed
    (CallFunction|DASHLocationCreator)
    (bind _dash_alpha (Timeline|TL_Dash PlayFromStart)
      (:Update
        (Transformation|SetActorLocation (Math|Vector|Lerp(Vector) (Variables|Default|GetCurrentLocation) (Variables|Default|GetDashLocation) _dash_alpha) false false)))))

(event Input|ActionEvents|InputActionADS
  (params (Key :type Key%20Structure))
  ;[0.15 0.15 0.15 0.5] ACTIONS
  (:Pressed
    (Class|PrimitiveComponent|SetOwnerNoSee (Variables|Character|GetMesh) true)
    (bind _asbp_player_controller (Utilities|Casting|CastToBP_PlayerController (Pawn|GetController)))
    (Default|EnterADS (Variables|/Game/SS_SNIPERGAME/SS_BLUEPRINTS/BP_PlayerController.BP_PlayerController_C|GetPlayerCamera _asbp_player_controller)))
  (:Released
    (Class|PrimitiveComponent|SetOwnerNoSee (Variables|Character|GetMesh) false)
    (bind _asbp_player_controller_2 (Utilities|Casting|CastToBP_PlayerController (Pawn|GetController)))
    (Default|ExitADS (Variables|/Game/SS_SNIPERGAME/SS_BLUEPRINTS/BP_PlayerController.BP_PlayerController_C|GetPlayerCamera _asbp_player_controller_2))))

(event Input|AxisEvents|InputAxisUP_DOWN
  (params (AxisValue :type Float%20%28single-precision%29))
  (bind _returnvalue (Pawn|GetControlRotation :!class /Script/Engine.Pawn))
  (bind (_roll _pitch _yaw) (Math|Rotator|BreakRotator _returnvalue))
  ;[0.15 0.15 0.15 0.5] PLAYER MOVEMENT
  (Pawn|Input|AddMovementInput (Math|Vector|GetForwardVector (Math|Rotator|MakeRotator _roll _pitch _yaw)) AxisValue false))

(event Input|AxisEvents|InputAxisLEFT_RIGHT
  (params (AxisValue :type Float%20%28single-precision%29))
  (bind _returnvalue (Pawn|GetControlRotation :!class /Script/Engine.Pawn))
  (bind (_roll _pitch _yaw) (Math|Rotator|BreakRotator _returnvalue))
  ;[0.15 0.15 0.15 0.5] PLAYER MOVEMENT
  (Pawn|Input|AddMovementInput (Math|Vector|GetRightVector (Math|Rotator|MakeRotator _roll _pitch _yaw)) AxisValue false))

(event Input|AxisEvents|InputAxisLOOK_LEFT_RIGHT
  (params (AxisValue :type Float%20%28single-precision%29))
  ;[0.15 0.15 0.15 0.5] LOOK
  (Pawn|Input|AddControllerYawInput AxisValue))

(event Input|AxisEvents|InputAxisLOOK_UP_DOWN
  (params (AxisValue :type Float%20%28single-precision%29))
  ;[0.15 0.15 0.15 0.5] LOOK
  (Pawn|Input|AddControllerPitchInput AxisValue))

(fn ConstructionScript)

(fn FIREBullet
  (bind _self self)
  (bind _projectilespawn (Variables|Default|GetProjectileSpawn))
  (bind _returnvalue (Transformation|GetWorldLocation _projectilespawn))
  (bind _asbp_player_controller (Utilities|Casting|CastToBP_PlayerController (Pawn|GetController)))
  (Class|CameraComponent|GetCameraView (Variables|/Game/SS_SNIPERGAME/SS_BLUEPRINTS/BP_PlayerCamera.BP_PlayerCamera_C|Get3rd_Person (Variables|/Game/SS_SNIPERGAME/SS_BLUEPRINTS/BP_PlayerController.BP_PlayerController_C|GetPlayerCamera _asbp_player_controller)) 0.0)
  (Variables|Default|SetCameraMaxRange (+ (Transformation|GetWorldLocation (Variables|/Game/SS_SNIPERGAME/SS_BLUEPRINTS/BP_PlayerCamera.BP_PlayerCamera_C|Get3rd_Person (Variables|/Game/SS_SNIPERGAME/SS_BLUEPRINTS/BP_PlayerController.BP_PlayerController_C|GetPlayerCamera _asbp_player_controller))) (* (Math|Vector|GetForwardVector (Variables|/Game/SS_SNIPERGAME/SS_BLUEPRINTS/BP_PlayerCamera.BP_PlayerCamera_C|Get3rd_Person (Variables|/Game/SS_SNIPERGAME/SS_BLUEPRINTS/BP_PlayerController.BP_PlayerController_C|GetPlayerCamera _asbp_player_controller))) 1e+05)))
  (bind (_outhit _returnvalue_2) (Collision|LineTraceByChannel (Transformation|GetWorldLocation (Variables|/Game/SS_SNIPERGAME/SS_BLUEPRINTS/BP_PlayerCamera.BP_PlayerCamera_C|Get3rd_Person (Variables|/Game/SS_SNIPERGAME/SS_BLUEPRINTS/BP_PlayerController.BP_PlayerController_C|GetPlayerCamera _asbp_player_controller))) (+ (Transformation|GetWorldLocation (Variables|/Game/SS_SNIPERGAME/SS_BLUEPRINTS/BP_PlayerCamera.BP_PlayerCamera_C|Get3rd_Person (Variables|/Game/SS_SNIPERGAME/SS_BLUEPRINTS/BP_PlayerController.BP_PlayerController_C|GetPlayerCamera _asbp_player_controller))) (* (Math|Vector|GetForwardVector (Variables|/Game/SS_SNIPERGAME/SS_BLUEPRINTS/BP_PlayerCamera.BP_PlayerCamera_C|Get3rd_Person (Variables|/Game/SS_SNIPERGAME/SS_BLUEPRINTS/BP_PlayerController.BP_PlayerController_C|GetPlayerCamera _asbp_player_controller))) 1e+05)) "TraceTypeQuery1" false 0 "ForDuration" true "(R=1.000000,G=0.000000,B=0.000000,A=1.000000)" "(R=0.000000,G=1.000000,B=0.000000,A=1.000000)" 2.0))
  (Rendering|Debug|DrawDebugSphere _returnvalue 8.0 12 "(R=1.000000,G=1.000000,B=1.000000,A=1.000000)" 5.0)
  (bind _returnvalue_3 (Game|SpawnActorfromClass "/Game/SS_SNIPERGAME/SS_BLUEPRINTS/BP_Bullet.BP_Bullet_C" (Math|Transform|MakeTransform _returnvalue (Math|Rotator|FindLookatRotation _returnvalue (Math|Vector|SelectVector (.ImpactPoint (Collision|BreakHitResult _outhit)) (Variables|Default|GetCameraMaxRange) _returnvalue_2))) "Undefined" "MultiplyWithRoot" _self _self))
  (Variables|Default|SetActiveBullet _returnvalue_3))

(fn PlayerDefaults
  (bind _capsulecomponent (Variables|Collision|GetCapsuleComponent))
  (Utilities|FlowControl|Sequence
    (:then_0
      (Input|EnableInput (Game|GetPlayerController 0))
      (Collision|SetCollisionEnabled _capsulecomponent "QueryAndPhysics")
      (Physics|SetSimulatePhysics _capsulecomponent false))
    (:then_1
      (CallFunction|SpawnWeapon (Variables|Default|GetEquipped%20Weapon%20to%20Spawn) "/Game/SS_SNIPERGAME/SS_BLUEPRINTS/BP_Scope.BP_Scope_C"))))

(fn SpawnWeapon
  (params (Weapon%20to%20Spawn :type BP%20Weapon%20Class%20Class%20Reference) (Scope%20Mesh :type BP%20Scope%20Attachment%20Class%20Class%20Reference))
  (bind _returnvalue (Game|SpawnActorfromClass Weapon%20to%20Spawn (Transformation|GetWorldTransform (Variables|Character|GetMesh)) "Undefined" "MultiplyWithRoot" 0 Scope%20Mesh 0))
  (bind _output_get (Variables|Default|SetEquipped%20Weapon _returnvalue))
  (Transformation|AttachComponentToComponent _output_get (Variables|Character|GetMesh) (Variables|/Game/SS_SNIPERGAME/SS_DATA/DA_WeaponData.DA_WeaponData_C|GetBone%20Socket%20Name (Variables|/Game/SS_SNIPERGAME/SS_DATA/BP_WeaponClass.BP_WeaponClass_C|GetGun%20Data _output_get)) "SnapToTarget" "SnapToTarget" "SnapToTarget" true)
  (return))

(fn DASHLocationCreator
  (bind _returnvalue (Class|Pawn|GetLastMovementInputVector))
  (bind (_x _y) (Math|Vector|BreakVector _returnvalue))
  (bind _output_get (Variables|Default|SetCurrentLocation (Transformation|GetActorLocation)))
  (Variables|Default|SetDashLocation (+ _output_get (* (Math|Vector|Normalize (Math|Vector|MakeVector _x _y 0.0)) (Variables|Default|GetDashDistance)))))

(fn ActorREF
  (bind _mesh (Variables|Character|GetMesh))
  (return self (Components|SkeletalMesh|GetAnimInstance _mesh) _mesh (Variables|Default|GetGameplay%20Tags)))
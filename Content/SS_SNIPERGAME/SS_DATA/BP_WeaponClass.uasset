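; Base weapon Blueprint for a sniper game that sets up the scope attachment and aim type on BeginPlay.
; It spawns the scope at the player character mesh's transform and snaps it to the weapon mesh's scope socket, if both scope and socket exist.
; Gameplay tags track the attachment state, and Aim.Scope is added when the exact Attachment.Scope tag is absent.
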(event EventBeginPlay
  (|SetAttachmentMeshandattachittoweapon)
  (|SetAimType))

(fn ConstructionScript)